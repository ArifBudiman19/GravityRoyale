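; CubePower is an indoor actor that spins six very bright, randomly colored spotlights, like a rotating light cube.
; The construction script passes each spotlight through SetupLight, which derives its color from random unit vectors and sets a fixed intensity.
; On BeginPlay, the authority tilts the actor, randomizes its yaw and picks a random Speed.
; Tick adds local yaw rotation scaled by Speed and delta time.
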(event EventTick
  (params (DeltaSeconds :type Float%20%28single-precision%29))
  (Transformation|AddActorLocalRotation (Math|Rotator|MakeRotator 0.0 0.0 (* DeltaSeconds (Variables|Default|GetSpeed))) false false))

(event EventBeginPlay
  (Networking|SwitchHasAuthority
    (:Authority
      (Transformation|SetActorRotation (Math|Rotator|MakeRotator 45.0 45.0 (Math|Random|RandomFloatinRange 0.0 3.6e+02)))
      (Variables|Default|SetSpeed (Math|Random|RandomFloatinRange 1e+02 2e+02)))))

(fn ConstructionScript
  (CallFunction|SetupLight (Variables|Default|GetSpotLight))
  (CallFunction|SetupLight (Variables|Default|GetSpotLight1))
  (CallFunction|SetupLight (Variables|Default|GetSpotLight2))
  (CallFunction|SetupLight (Variables|Default|GetSpotLight3))
  (CallFunction|SetupLight (Variables|Default|GetSpotLight4))
  (CallFunction|SetupLight (Variables|Default|GetSpotLight5)))

(fn SetupLight
  (params (Light :type Light%20Component%20Object%20Reference))
  (bind _returnvalue (Math|Random|RandomUnitVector))
  (bind _returnvalue_2 (Math|Vector|ClampVectorSize _returnvalue 0.8 1.0))
  (bind _returnvalue_3 (* _returnvalue_2 255.0))
  (Rendering|Components|Light|SetLightColor Light (Utilities|Struct|MakeLinearColor (.x _returnvalue_3) (.y _returnvalue_3) (.z _returnvalue_3) 1.0) true)
  (Rendering|Components|Light|SetIntensity Light 999999.0))