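; GravityController is a player controller that handles respawn requests and the in-game menu.
; Respawn, when no valid pawn is controlled, calls RequestForRespawn, which on authority asks GravityGameMode to respawn this controller.
; The local controller creates MenuWBP at BeginPlay, and the GameMenu input toggles it, switching cursor visibility and input mode between UI-only and game-only.
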(event Custom|HideMenu
  (Widget|RemovefromParent (Variables|Default|GetMenuWBP))
  (Input|SetInputModeGameOnly self)
  (Variables|Default|SetbShowMouseCursor false))

(event Custom|RequestForRespawn
  (bind _returnvalue (Game|GetGameMode))
  (Networking|SwitchHasAuthority
    (:Authority
      (Utilities|IsValid _returnvalue
        (:Is%20Valid
          (bind _asgravity_game_mode (Utilities|Casting|CastToGravityGameMode _returnvalue))
          (Utilities|IsValid _asgravity_game_mode
            (:Is%20Valid
              (Default|Respawn _asgravity_game_mode self))))))))

(event Custom|Respawn
  (Utilities|IsValid (Pawn|GetControlledPawn self)
    (:Is%20Not%20Valid
      (CallFunction|RequestforRespawn))))

(event Custom|ToggleMenu
  (bind _self self)
  (bind _menuwbp (Variables|Default|GetMenuWBP))
  (bind _menuwbp_2 (Variables|Default|GetMenuWBP))
  (Utilities|IsValid _menuwbp
    (:Is%20Valid
      (if (UserInterface|Viewport|IsinViewport _menuwbp)
        (Widget|RemovefromParent _menuwbp_2)
        (Input|SetInputModeGameOnly _self)
        (Variables|Default|SetbShowMouseCursor false)
        (else
          (UserInterface|Viewport|AddtoViewport _menuwbp_2 0)
          (Input|SetInputModeUIOnly _self (Variables|Default|GetMenuWBP) "DoNotLock")
          (Variables|Default|SetbShowMouseCursor true))))))

(event EventBeginPlay
  (if (Pawn|IsLocalController)
    (bind _returnvalue (UserInterface|CreateWidget "/Game/Blueprint/Gravity/MenuWBP.MenuWBP_C" self))
    (Variables|Default|SetMenuWBP _returnvalue)))

(event Input|ActionEvents|InputActionGameMenu
  (params (Key :type Key%20Structure))
  (:Pressed
    (CallFunction|ToggleMenu)))

(fn ConstructionScript)