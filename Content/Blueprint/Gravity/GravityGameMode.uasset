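; GravityGameMode is a game mode Blueprint that respawns players in the Gravity game.
; Its Respawn event, on authority with a valid controller, spawns the default pawn at a randomly indexed PlayerStart, possesses it, then has GravityGameInstance create a crosshair for it.
; The random index uses RandomInteger of the array length minus one, so the last PlayerStart found is never picked when several exist.
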(event Custom|Respawn
  (params (Controller :type Player%20Controller%20Object%20Reference))
  (Utilities|IsValid Controller
    (:Is%20Valid
      (Networking|SwitchHasAuthority
        (:Authority
          (bind _outactors (Actor|GetAllActorsOfClass "/Script/Engine.PlayerStart"))
          (bind _returnvalue (Game|SpawnActorfromClass (Variables|Default|GetDefaultPawnClass) (Transformation|GetActorTransform (Utilities|Array|Get(acopy) _outactors (Math|Random|RandomInteger (- (Utilities|Array|Length _outactors) 1)))) "Undefined" 0 0))
          (Utilities|IsValid _returnvalue
            (:Is%20Valid
              (Pawn|Possess Controller _returnvalue)
              (bind _asgravity_game_instance (Utilities|Casting|CastToGravityGameInstance (Game|GetGameInstance)))
              (Default|CreateCrosshair _asgravity_game_instance _returnvalue))))))))

(fn ConstructionScript)