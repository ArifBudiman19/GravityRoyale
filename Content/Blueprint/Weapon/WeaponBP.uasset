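; Networked hitscan weapon base that fires on a looping timer derived from rate of fire, with drop support and empty aim events.
; Fire routes remote calls to the server, which line-traces from the owner's view within a spread cone and applies point damage.
; The server then sets a replicated trace struct, whose OnRep replays muzzle, tracer, camera shake and impact effects on clients.
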(event Custom|ServerFire
  (CallFunction|Fire))

(event Custom|StartFire
  (Utilities|FlowControl|DoOnce false :!label _label
    (:Completed
      (bind _returnvalue (Utilities|Time|SetTimerbyFunctionName 0 "Fire" (Variables|Default|GetTimeBetweenShots) true))
      (Variables|Default|SetTimerHandleBetweenShots _returnvalue)
      (Utilities|FlowControl|Delay (Math|Float|Max(Float) (- (+ (Variables|Default|GetLastFireTime) (Variables|Default|GetTimeBetweenShots)) (Utilities|Time|GetTimeSeconds)) 0.0))
      (goto _label Reset))))

(event Custom|StopFire
  (bind _timerhandlebetweenshots (Variables|Default|GetTimerHandleBetweenShots))
  (if (Utilities|Time|IsValidTimerHandle _timerhandlebetweenshots)
    (Utilities|Time|ClearandInvalidateTimerbyHandle _timerhandlebetweenshots)))

(event Custom|StartAim)

(event Custom|StopAim)

(event Custom|Fire
  (bind _returnvalue (Components|GetOwner))
  (bind _returnvalue_2 (Components|GetOwner))
  (bind _returnvalue_3 (Utilities|GetMuzzleLocation))
  ;[1 1 1] Fire
  (Networking|SwitchHasAuthority
    (:Authority
      (Utilities|IsValid _returnvalue_2
        (:Is%20Valid
          (bind (_out _forward) (Class|ICharacter|GetViewForward(Message) _returnvalue_2))
          (bind (_outhit _returnvalue_4) (Collision|LineTraceByChannel (+ _out (* (Class|KismetMathLibrary|RandomUnitVectorinConeinRadians _forward (Math|Trig|DegreesToRadians (Variables|Weapon|GetBulletSpread))) (Variables|Weapon|GetOffset))) (+ _out (* (Class|KismetMathLibrary|RandomUnitVectorinConeinRadians _forward (Math|Trig|DegreesToRadians (Variables|Weapon|GetBulletSpread))) (Variables|Weapon|GetRange))) "TraceTypeQuery4" false 0 "None" true "(R=1.000000,G=0.000000,B=0.000000,A=1.000000)" "(R=0.000000,G=1.000000,B=0.000000,A=1.000000)" 3.0))
          (if _returnvalue_4
            (Game|Damage|ApplyPointDamage (.HitActor (Collision|BreakHitResult _outhit)) (* (Variables|Weapon|GetBaseDamage) (Utilities|Select :Index (Collision|GetSurfaceType _outhit) :SurfaceType_Default 1.0)) _forward _outhit (Game|GetInstigatorController _returnvalue) _returnvalue (Variables|Weapon|GetDamageType)))
          (CallFunction|SpawnFireEffect (Utilities|GetMuzzleLocation) (select _returnvalue_4 (.ImpactPoint (Collision|BreakHitResult _outhit)) (+ _out (* (Class|KismetMathLibrary|RandomUnitVectorinConeinRadians _forward (Math|Trig|DegreesToRadians (Variables|Weapon|GetBulletSpread))) (Variables|Weapon|GetRange)))))
          (Networking|SwitchHasAuthority
            (:Authority
              (Variables|Default|SetHitScanTrace (Utilities|Struct|MakeHitScanTrace (Collision|GetSurfaceType _outhit) (Math|Vector|MakeVectorNetQuantize (.x _returnvalue_3) (.y _returnvalue_3) (.z _returnvalue_3)) (Math|Vector|MakeVectorNetQuantize (.X (Math|Vector|BreakVector (select _returnvalue_4 (.ImpactPoint (Collision|BreakHitResult _outhit)) (+ _out (* (Class|KismetMathLibrary|RandomUnitVectorinConeinRadians _forward (Math|Trig|DegreesToRadians (Variables|Weapon|GetBulletSpread))) (Variables|Weapon|GetRange)))))) (.Y (Math|Vector|BreakVector (select _returnvalue_4 (.ImpactPoint (Collision|BreakHitResult _outhit)) (+ _out (* (Class|KismetMathLibrary|RandomUnitVectorinConeinRadians _forward (Math|Trig|DegreesToRadians (Variables|Weapon|GetBulletSpread))) (Variables|Weapon|GetRange)))))) (.Z (Math|Vector|BreakVector (select _returnvalue_4 (.ImpactPoint (Collision|BreakHitResult _outhit)) (+ _out (* (Class|KismetMathLibrary|RandomUnitVectorinConeinRadians _forward (Math|Trig|DegreesToRadians (Variables|Weapon|GetBulletSpread))) (Variables|Weapon|GetRange))))))))))))))
    (:Remote
      (CallFunction|ServerFire))))

(event Custom|Drop
  (Utilities|IsValid (Components|GetOwner)
    (:Is%20Valid
      (Actor|SetOwner 0)
      (Transformation|DetachFromActor "KeepRelative" "KeepRelative" "KeepRelative"))))

(event EventBeginPlay
  (Variables|Default|SetTimeBetweenShots (/ 6e+01 (Variables|Weapon|GetRateOfFire))))

(fn ConstructionScript)

(fn OnRepHitScanTrace
  (bind _hitscantrace (Variables|Default|GetHitScanTrace))
  (CallFunction|SpawnFireEffect (.tracefrom _hitscantrace) (.traceend _hitscantrace))
  (CallFunction|SpawnImpactEffect (.surfacetype _hitscantrace) (.tracefrom _hitscantrace) (.traceend _hitscantrace)))

(fn SpawnFireEffect
  (params (MuzzleLocation :type Vector) (TraceEndLocation :type Vector))
  (bind _muzzleeffect (Variables|Weapon|GetMuzzleEffect))
  (bind _tracereffect (Variables|Weapon|GetTracerEffect))
  (Utilities|FlowControl|Sequence
    (:then_0
      (Utilities|IsValid _muzzleeffect
        (:Is%20Valid
          (Effects|SpawnEmitterAttached _muzzleeffect (Variables|Components|GetMeshComponent) (Variables|Weapon|GetMuzzleSocketName)))))
    (:then_1
      (Utilities|IsValid _tracereffect
        (:Is%20Valid
          (bind _returnvalue (Effects|SpawnEmitteratLocation _tracereffect MuzzleLocation))
          (Effects|Components|ParticleSystem|SetVectorParameter _returnvalue (Variables|Weapon|GetTracerTargetName) TraceEndLocation))))
    (:then_2
      (bind _aspawn (Utilities|Casting|CastToPawn (Components|GetOwner)))
      (if (!= (Variables|Weapon|GetFireCameraShake) 0)
        (bind _asplayer_controller (Utilities|Casting|CastToPlayerController (Pawn|GetController _aspawn)))
        (Class|PlayerController|ClientPlayCameraShake _asplayer_controller (Variables|Weapon|GetFireCameraShake) 1.0 "CameraLocal" "0, 0, 0")))
    (:then_3
      (Variables|Default|SetNetUpdateFrequency 66.0)
      (Variables|Default|SetMinNetUpdateFrequency 33.0))))

(fn SpawnImpactEffect
  (params (SurfaceType :type EPhysicalSurface%20Enum :default "SurfaceType_Default") (ImpactPoint :type Vector) (TraceFrom :type Vector))
  (Utilities|FlowControl|Sequence
    (:then_0
      (switch Utilities|FlowControl|Switch|SwitchonEPhysicalSurface SurfaceType
        (:SurfaceType_Default
          (LocalVariables|SetImpactEffect (Variables|Weapon|GetDefaultImpactEffect)))))
    (:then_1
      (Utilities|IsValid (LocalVariables|GetImpactEffect)
        (:Is%20Valid
          (Effects|SpawnEmitteratLocation (LocalVariables|GetImpactEffect) ImpactPoint (Class|KismetMathLibrary|QuatRotator (Class|KismetMathLibrary|ToQuaterion(Vector) (Math|Vector|Normalize (- ImpactPoint TraceFrom))))))))))