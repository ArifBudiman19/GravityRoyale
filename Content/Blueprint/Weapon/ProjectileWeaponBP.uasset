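; Projectile weapon Blueprint whose Fire event spawns a replicated-movement projectile on the authority.
; Fire line-traces from the owner's view with random cone spread, then aims the projectile from the muzzle at the impact point, or along a random spread direction on a miss.
; SpawnFireEffect attaches the muzzle emitter, plays a camera shake through the owning player controller and sets net update frequencies.
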(event EventBeginPlay
  (|CallParentFunction) ; This node is disabled and will not be called.\nDrag off pins to build functionality.
)

(event EventFire
  (bind _returnvalue (Components|GetOwner))
  (bind _returnvalue_2 (Utilities|GetMuzzleLocation))
  (Networking|SwitchHasAuthority
    (:Authority
      (Utilities|IsValid _returnvalue
        (:Is%20Valid
          (bind (_out _forward) (Class|ICharacter|GetViewForward(Message) _returnvalue))
          (CallFunction|SpawnFireEffect (Utilities|GetMuzzleLocation) "0, 0, 0")
          (bind (_outhit _returnvalue_3) (Collision|LineTraceByChannel (+ _out (* (Class|KismetMathLibrary|RandomUnitVectorinConeinRadians _forward (Math|Trig|DegreesToRadians (Variables|Default|GetBulletSpread))) (Variables|Default|GetOffset))) (+ _out (* (Class|KismetMathLibrary|RandomUnitVectorinConeinRadians _forward (Math|Trig|DegreesToRadians (Variables|Default|GetBulletSpread))) (Variables|Default|GetRange))) "TraceTypeQuery1" false 0 "None" true "(R=1.000000,G=0.000000,B=0.000000,A=1.000000)" "(R=0.000000,G=1.000000,B=0.000000,A=1.000000)" 1e+01))
          (bind _returnvalue_4 (Game|SpawnActorfromClass (Variables|Weapon|GetProjectileClass) (Math|Transform|MakeTransform _returnvalue_2 (select _returnvalue_3 (Math|Rotator|FindLookatRotation _returnvalue_2 (.ImpactPoint (Collision|BreakHitResult _outhit))) (Math|Rotator|FindLookatRotation (Utilities|GetMuzzleLocation) (* (Class|KismetMathLibrary|RandomUnitVectorinConeinRadians _forward (Math|Trig|DegreesToRadians (Variables|Default|GetBulletSpread))) (Variables|Default|GetRange))))) "Undefined" (Components|GetOwner) 0))
          (Class|Actor|SetReplicateMovement _returnvalue_4 true))))))

(event EventSpawnFireEffect
  (params (MuzzleLocation :type Vector :default "0, 0, 0") (TraceEndLocation :type Vector :default "0, 0, 0"))
  (bind _muzzleeffect (Variables|Default|GetMuzzleEffect))
  (Utilities|FlowControl|Sequence
    (:then_0
      (Utilities|IsValid _muzzleeffect
        (:Is%20Valid
          (Effects|SpawnEmitterAttached _muzzleeffect (Variables|Default|GetMeshComponent) (Variables|Default|GetMuzzleSocketName)))))
    (:then_1
      (bind _aspawn (Utilities|Casting|CastToPawn (Components|GetOwner)))
      (if (!= (Variables|Default|GetFireCameraShake) 0)
        (bind _asplayer_controller (Utilities|Casting|CastToPlayerController (Pawn|GetController _aspawn)))
        (Class|PlayerController|ClientPlayCameraShake _asplayer_controller (Variables|Default|GetFireCameraShake) 1.0 "CameraLocal" "0, 0, 0")))
    (:then_2
      (Variables|Default|SetNetUpdateFrequency 66.0)
      (Variables|Default|SetMinNetUpdateFrequency 33.0))))

(fn ConstructionScript
  (|CallParentFunction))