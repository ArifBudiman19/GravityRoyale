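; Health component that tracks an actor's health, damage, healing and death state.
; On the authority, BeginPlay binds to the owner's any-damage event, which clamps health, flags death at zero and broadcasts OnHealthChanged.
; Heal restores clamped health while alive and broadcasts the same delegate with negative damage.
; The component's own authority-bound OnHealthChanged handler is empty.
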(event Custom|HandleDamage
  (params (DamagedActor :type Actor%20Object%20Reference) (Damage :type Float%20%28single-precision%29) (DamageType :type Damage%20Type%20Object%20Reference) (InstigatedBy :type Controller%20Object%20Reference) (DamageCauser :type Actor%20Object%20Reference))
  (if (not (or (<= (Variables|Default|GetInitialHealth) 0.0) (Variables|Default|GetIsDead)))
    (bind _output_get (Variables|Default|SetHealth (Math|Float|Clamp(Float) (- (Variables|Default|GetHealth) Damage) 0.0 (Variables|Default|GetInitialHealth))))
    (Variables|Default|SetIsDead (<= _output_get 0.0))
    (Default|CallOnHealthChanged _output_get Damage DamageType InstigatedBy DamageCauser)))

(event Custom|OnHealthChanged_Event
  (params (Health :type Float%20%28single-precision%29) (Damage :type Float%20%28single-precision%29) (DamageType :type Damage%20Type%20Object%20Reference) (InstigatedBy :type Controller%20Object%20Reference) (DamageCauser :type Actor%20Object%20Reference)))

(event EventBeginPlay
  (bind _returnvalue (Components|GetOwner))
  (Variables|Default|SetHealth (Variables|Default|GetInitialHealth))
  (if (Ability|HasAuthority _returnvalue)
    (EventDispatchers|BindEventtoOnTakeAnyDamage _returnvalue (delegate Custom|HandleDamage))
    (EventDispatchers|BindEventtoOnHealthChanged (delegate Custom|OnHealthChanged_Event))))

(fn GetHealth
  (return (Variables|Default|GetHealth)))

(fn Heal
  (params (Amount :type Float%20%28single-precision%29))
  (if (not (Variables|Default|GetIsDead))
    (bind _output_get (Variables|Default|SetHealth (Math|Float|Clamp(Float) (+ Amount (Variables|Default|GetHealth)) 0.0 (Variables|Default|GetInitialHealth))))
    (Default|CallOnHealthChanged _output_get (* Amount -1.0))))