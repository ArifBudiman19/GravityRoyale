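; Actor component that gives its owner planet-style gravity by pulling it toward the surfaces of tracked planet actors.
; While the list is empty, a line trace sweeps by rotating one degree of roll per tick and adds any hit actor as a planet.
; Otherwise, each tick traces toward every planet and adds velocity to the root primitive against the impact normal, without delta-time scaling.
; AddPlanet and RemovePlanet edit the list.
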(event EventTick
  (params (DeltaSeconds :type Float%20%28single-precision%29))
  (bind _returnvalue (Components|GetOwner))
  (bind _returnvalue_2 (Components|GetOwner))
  (bind _returnvalue_3 (Transformation|GetActorLocation _returnvalue))
  (if (< (Utilities|Array|Length (Variables|Default|GetPlanets)) 1)
    (Utilities|FlowControl|Sequence
      (:then_0
        (bind (_outhit _returnvalue_4) (Collision|LineTraceByChannel _returnvalue_3 (+ _returnvalue_3 (* (Math|Vector|RotateVector (Transformation|GetActorUpVector _returnvalue) (Math|Rotator|MakeRotator (Variables|Default|GetAngle) 0.0 0.0)) (* -1.0 (Variables|Default|GetTraceLength)))) "TraceTypeQuery3" false 0 "None" true "(R=1.000000,G=0.000000,B=0.000000,A=1.000000)" "(R=0.000000,G=1.000000,B=0.000000,A=1.000000)" 1.0))
        (if _returnvalue_4
          (Utilities|Array|AddUnique (Variables|Default|GetPlanets) (.HitActor (Collision|BreakHitResult _outhit)))))
      (:then_1
        (bind _result (Math|Float|IncrementFloat (Variables|Default|GetAngle))
          (:%20%20
            (if (>= _result 3.6e+02)
              (Variables|Default|SetAngle 0.0))))))
    (else
      (for _array_element (Variables|Default|GetPlanets)
        (Utilities|IsValid _returnvalue_2
          (:Is%20Valid
            (bind (_outhit_2 _returnvalue_5) (Collision|LineTraceByChannel (Transformation|GetActorLocation _returnvalue_2) (Transformation|GetActorLocation _array_element) "TraceTypeQuery3" false 0 "None"))
            (if _returnvalue_5
              (bind _asprimitive_component (Utilities|Casting|CastToPrimitiveComponent (Variables|/Script/Engine.Actor|GetRootComponent (Components|GetOwner))))
              (Physics|SetPhysicsLinearVelocity _asprimitive_component (* (.ImpactNormal (Collision|BreakHitResult _outhit_2)) (* (Variables|Default|GetGravityStrength) -1.0)) true "None"))))))))

(fn AddPlanet
  (params (Planet :type Actor%20Object%20Reference))
  (bind _returnvalue (Utilities|Array|AddUnique (Variables|Default|GetPlanets) Planet))
  (return _returnvalue))

(fn RemovePlanet
  (params (Planet :type Actor%20Object%20Reference))
  (bind _returnvalue (Utilities|Array|RemoveItem (Variables|Default|GetPlanets) Planet))
  (return _returnvalue))