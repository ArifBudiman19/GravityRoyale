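; LobbyController is a player controller for the lobby that shows the lobby menu to the local player.
; On BeginPlay, only for the local controller, it creates the LobbyWBP widget, stores it as MainMenuWBP and adds it to the viewport.
; It then shows the mouse cursor and switches input to UI-only, focused on that widget without locking the mouse.
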(event EventBeginPlay
  (if (Pawn|IsLocalController)
    (bind _returnvalue (UserInterface|CreateWidget "/Game/Blueprint/Lobby/LobbyWBP.LobbyWBP_C" self))
    (bind _output_get (Variables|Default|SetMainMenuWBP _returnvalue))
    (Utilities|IsValid _output_get
      (:Is%20Valid
        (if (not (UserInterface|Viewport|IsinViewport _output_get))
          (UserInterface|Viewport|AddtoViewport (Variables|Default|GetMainMenuWBP) 0))
        (Variables|Default|SetbShowMouseCursor true)
        (Input|SetInputModeUIOnly self (Variables|Default|GetMainMenuWBP) "DoNotLock")))))

(fn ConstructionScript)